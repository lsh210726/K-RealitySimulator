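; Demo actor for the SimpleUI widgets that opens one of six popups, chosen by UIStateNum, when its collision box is overlapped.
; BeginPlay creates all widgets; overlap begin and end show or remove the selected one and switch cursor and input mode.
; Tick polls button presses instead of binding click events.
; The Setting popup live-previews cube scale, material, rotation and visibility, with helper functions to load, save or default values.
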(event OnComponentBeginOverlap(CubeCollision)
  (params (OverlappedComponent :type Primitive%20Component%20Object%20Reference) (OtherActor :type Actor%20Object%20Reference) (OtherComp :type Primitive%20Component%20Object%20Reference) (OtherBodyIndex :type Integer) (bFromSweep :type Boolean) (SweepResult :type Hit%20Result%20Structure%20%28by%20ref%29))
  (bind _returnvalue (Game|GetPlayerController 0))
  (bind _returnvalue_2 (Game|GetPlayerController 0))
  (bind _returnvalue_3 (Game|GetPlayerController 0))
  (bind _returnvalue_4 (Game|GetPlayerController 0))
  (bind _returnvalue_5 (Game|GetPlayerController 0))
  (bind _returnvalue_6 (Game|GetPlayerController 0))
  (bind _textinput (Variables|Default|GetTextInput))
  ;[1 1 1] Overlap Begin Event _ Open widgets and add to user's viewport
  (switch int (Variables|Default|GetUIStateNum)
    (:0
      ;[1 1 1] 0_NotificationCommon
      (UserInterface|Viewport|AddtoViewport (Variables|Default|GetNotificationCommon) 0)
      (Variables|/Script/Engine.PlayerController|SetbShowMouseCursor _returnvalue true)
      (Audio|PlaySound2D "/Game/SimpleUI/Sound/S_Popup_Cue.S_Popup_Cue")
      (Input|SetInputModeGameandUI _returnvalue 0 "DoNotLock" false))
    (:1
      ;[1 1 1] 1_Notification_Success
      (UserInterface|Viewport|AddtoViewport (Variables|Default|GetNotificationSuccess) 0)
      (Variables|/Script/Engine.PlayerController|SetbShowMouseCursor _returnvalue_6 true)
      (Audio|PlaySound2D "/Game/SimpleUI/Sound/S_Success_Cue.S_Success_Cue")
      (Input|SetInputModeGameandUI _returnvalue_6 0 "DoNotLock" false))
    (:2
      ;[1 1 1] 2_Notfication_Warning
      (UserInterface|Viewport|AddtoViewport (Variables|Default|GetNotificationWarning) 0)
      (Variables|/Script/Engine.PlayerController|SetbShowMouseCursor _returnvalue_5 true)
      (Audio|PlaySound2D "/Game/SimpleUI/Sound/S_Warning_Cue.S_Warning_Cue")
      (Input|SetInputModeGameandUI _returnvalue_5 0 "DoNotLock" false))
    (:3
      ;[1 1 1] 3_Scroll
      (UserInterface|Viewport|AddtoViewport (Variables|Default|GetScroll) 0)
      (Variables|/Script/Engine.PlayerController|SetbShowMouseCursor _returnvalue_4 true)
      (Audio|PlaySound2D "/Game/SimpleUI/Sound/S_Popup_Cue.S_Popup_Cue")
      (Input|SetInputModeGameandUI _returnvalue_4 0 "DoNotLock" false))
    (:4
      ;[1 1 1] 4_TextInput
      (Rendering|Components|TextRender|SetText (Variables|/Game/SimpleUI/Blueprint/WidgetBlueprint/WG_TextInput.WG_TextInput_C|GetTextBox _textinput) "")
      (UserInterface|Viewport|AddtoViewport _textinput 0)
      (Variables|/Script/Engine.PlayerController|SetbShowMouseCursor _returnvalue_3 true)
      (Audio|PlaySound2D "/Game/SimpleUI/Sound/S_Popup_Cue.S_Popup_Cue")
      (Input|SetInputModeGameandUI _returnvalue_3 0 "DoNotLock" false))
    (:5
      ;[1 1 1] 5_Setting
      (CallFunction|GetSettingCurrentValue)
      (UserInterface|Viewport|AddtoViewport (Variables|Default|GetSetting) 0)
      (Variables|/Script/Engine.PlayerController|SetbShowMouseCursor _returnvalue_2 true)
      (Audio|PlaySound2D "/Game/SimpleUI/Sound/S_Popup_Cue.S_Popup_Cue")
      (Input|SetInputModeGameandUI _returnvalue_2 0 "DoNotLock" false))))

(event OnComponentEndOverlap(CubeCollision)
  (params (OverlappedComponent :type Primitive%20Component%20Object%20Reference) (OtherActor :type Actor%20Object%20Reference) (OtherComp :type Primitive%20Component%20Object%20Reference) (OtherBodyIndex :type Integer))
  (bind _returnvalue (Game|GetPlayerController 0))
  (bind _returnvalue_2 (Game|GetPlayerController 0))
  (bind _returnvalue_3 (Game|GetPlayerController 0))
  (bind _returnvalue_4 (Game|GetPlayerController 0))
  (bind _returnvalue_5 (Game|GetPlayerController 0))
  (bind _returnvalue_6 (Game|GetPlayerController 0))
  ;[1 1 1] Overlap End Event _ Close widgets
  (switch int (Variables|Default|GetUIStateNum)
    (:0
      ;[1 1 1] 0_NotificationCommon
      (Widget|RemovefromParent (Variables|Default|GetNotificationCommon))
      (Variables|/Script/Engine.PlayerController|SetbShowMouseCursor _returnvalue_2 false)
      (Input|SetInputModeGameOnly _returnvalue_2))
    (:1
      ;[1 1 1] 1_Notification_Success
      (Widget|RemovefromParent (Variables|Default|GetNotificationSuccess))
      (Variables|/Script/Engine.PlayerController|SetbShowMouseCursor _returnvalue_6 false)
      (Input|SetInputModeGameOnly _returnvalue_6))
    (:2
      ;[1 1 1] 2_Notfication_Warning
      (Widget|RemovefromParent (Variables|Default|GetNotificationWarning))
      (Variables|/Script/Engine.PlayerController|SetbShowMouseCursor _returnvalue_5 false)
      (Input|SetInputModeGameOnly _returnvalue_5))
    (:3
      ;[1 1 1] 3_Scroll
      (Widget|RemovefromParent (Variables|Default|GetScroll))
      (Variables|/Script/Engine.PlayerController|SetbShowMouseCursor _returnvalue_4 false)
      (Input|SetInputModeGameOnly _returnvalue_4))
    (:4
      ;[1 1 1] 4_TextInput
      (Widget|RemovefromParent (Variables|Default|GetTextInput))
      (Variables|/Script/Engine.PlayerController|SetbShowMouseCursor _returnvalue_3 false)
      (Input|SetInputModeGameOnly _returnvalue_3))
    (:5
      ;[1 1 1] 5_Setting
      (Widget|RemovefromParent (Variables|Default|GetSetting))
      (Variables|/Script/Engine.PlayerController|SetbShowMouseCursor _returnvalue false)
      (Input|SetInputModeGameOnly _returnvalue))))

(event EventBeginPlay
  ;[1 1 1] Initial Setup
  (Utilities|FlowControl|Sequence
    (:then_0
      ;[1 1 1] 0_NotificationCommon
      (bind _returnvalue (UserInterface|CreateWidget "/Game/SimpleUI/Blueprint/WidgetBlueprint/WG_Notification_Common.WG_Notification_Common_C" (Game|GetPlayerController 0)))
      (Variables|Default|SetNotificationCommon _returnvalue))
    (:then_1
      ;[1 1 1] 1_Notification_Success
      (bind _returnvalue_2 (UserInterface|CreateWidget "/Game/SimpleUI/Blueprint/WidgetBlueprint/WG_Notification_Success.WG_Notification_Success_C" (Game|GetPlayerController 0)))
      (Variables|Default|SetNotificationSuccess _returnvalue_2))
    (:then_2
      ;[1 1 1] 2_Notfication_Warning
      (bind _returnvalue_3 (UserInterface|CreateWidget "/Game/SimpleUI/Blueprint/WidgetBlueprint/WG_Notification_Warning.WG_Notification_Warning_C" (Game|GetPlayerController 0)))
      (Variables|Default|SetNotificationWarning _returnvalue_3))
    (:then_3
      ;[1 1 1] 3_Scroll
      (bind _returnvalue_4 (UserInterface|CreateWidget "/Game/SimpleUI/Blueprint/WidgetBlueprint/WG_Scroll.WG_Scroll_C" (Game|GetPlayerController 0)))
      (Variables|Default|SetScroll _returnvalue_4))
    (:then_4
      ;[1 1 1] 4_TextInput
      (bind _returnvalue_5 (UserInterface|CreateWidget "/Game/SimpleUI/Blueprint/WidgetBlueprint/WG_TextInput.WG_TextInput_C" (Game|GetPlayerController 0)))
      (Variables|Default|SetTextInput _returnvalue_5))
    (:then_5
      ;[1 1 1] 5_Setting
      (bind _returnvalue_6 (UserInterface|CreateWidget "/Game/SimpleUI/Blueprint/WidgetBlueprint/WG_Setting.WG_Setting_C" (Game|GetPlayerController 0)))
      (Variables|Default|SetSetting _returnvalue_6)
      (CallFunction|GetSettingCurrentValue))
    (:then_6
      ;[1 1 1] Initial Setting For testing each UI
      (switch int (Variables|Default|GetUIStateNum)
        (:4
          (Development|SetHiddeninGame (Variables|Default|GetTextRender) false false)
          (Rendering|Components|TextRender|SetText (Variables|Default|GetTextRender) (Utilities|Text|ToText(String) "Input any text")))
        (:5
          (Development|SetHiddeninGame (Variables|Default|GetCube) false false))))))

(event EventTick
  (params (DeltaSeconds :type Float%20%28single-precision%29))
  (bind _returnvalue (Utilities|Time|GetWorldDeltaSeconds))
  (bind _returnvalue_2 (Game|GetPlayerController 0))
  (bind _returnvalue_3 (Game|GetPlayerController 0))
  (bind _returnvalue_4 (Game|GetPlayerController 0))
  (bind _returnvalue_5 (Game|GetPlayerController 0))
  (bind _returnvalue_6 (Game|GetPlayerController 0))
  (bind _returnvalue_7 (Game|GetPlayerController 0))
  (bind _returnvalue_8 (Game|GetPlayerController 0))
  (bind _returnvalue_9 (Game|GetPlayerController 0))
  (bind _returnvalue_10 (Game|GetPlayerController 0))
  (bind _returnvalue_11 (Game|GetPlayerController 0))
  (bind _returnvalue_12 (Game|GetPlayerController 0))
  (bind _returnvalue_13 (Game|GetPlayerController 0))
  (bind _cube (Variables|Default|GetCube))
  (bind _cube2 (Variables|Default|GetCube2))
  (bind _cube3 (Variables|Default|GetCube3))
  (bind _scroll (Variables|Default|GetScroll))
  (bind _cube2_2 (Variables|Default|GetCube2))
  (bind _cube3_2 (Variables|Default|GetCube3))
  (bind _notificationcommon (Variables|Default|GetNotificationCommon))
  (bind _notificationsuccess (Variables|Default|GetNotificationSuccess))
  (bind _notificationwarning (Variables|Default|GetNotificationWarning))
  (bind _textinput (Variables|Default|GetTextInput))
  (bind _cube_2 (Variables|Default|GetCube))
  (bind _textinput_2 (Variables|Default|GetTextInput))
  (bind _setting (Variables|Default|GetSetting))
  (bind _array (Utilities|Array|MakeArray _cube_2 _cube2_2 _cube3_2))
  (bind _array_2 (Utilities|Array|MakeArray _cube _cube2 _cube3))
  ;[1 1 1] For Interacting each components of widgets
  (switch int (Variables|Default|GetUIStateNum)
    (:0
      ;[1 1 1] 0_Notification Common
      (Utilities|FlowControl|Sequence
        (:then_0
          (if (Class|Button|IsPressed (Variables|/Game/SimpleUI/Blueprint/WidgetBlueprint/WG_Notification_Common.WG_Notification_Common_C|GetOKButton _notificationcommon))
            (Widget|RemovefromParent _notificationcommon)
            (Variables|/Script/Engine.PlayerController|SetbShowMouseCursor _returnvalue_2 false)
            (Audio|PlaySound2D "/Game/SimpleUI/Sound/S_Click_Cue.S_Click_Cue")
            (Input|SetInputModeGameOnly _returnvalue_2)))
        (:then_1
          (if (Class|Button|IsPressed (Variables|/Game/SimpleUI/Blueprint/WidgetBlueprint/WG_Notification_Common.WG_Notification_Common_C|GetCancelButton _notificationcommon))
            (Widget|RemovefromParent _notificationcommon)
            (Variables|/Script/Engine.PlayerController|SetbShowMouseCursor _returnvalue_12 false)
            (Audio|PlaySound2D "/Game/SimpleUI/Sound/S_Click_Cue.S_Click_Cue")
            (Input|SetInputModeGameOnly _returnvalue_12)))))
    (:1
      ;[1 1 1] 1_Notification Success
      (Utilities|FlowControl|Sequence
        (:then_0
          (if (Class|Button|IsPressed (Variables|/Game/SimpleUI/Blueprint/WidgetBlueprint/WG_Notification_Success.WG_Notification_Success_C|GetOKButton _notificationsuccess))
            (Widget|RemovefromParent _notificationsuccess)
            (Variables|/Script/Engine.PlayerController|SetbShowMouseCursor _returnvalue_5 false)
            (Audio|PlaySound2D "/Game/SimpleUI/Sound/S_Click_Cue.S_Click_Cue")
            (Input|SetInputModeGameOnly _returnvalue_5)))
        (:then_1
          (if (Class|Button|IsPressed (Variables|/Game/SimpleUI/Blueprint/WidgetBlueprint/WG_Notification_Success.WG_Notification_Success_C|GetCancelButton _notificationsuccess))
            (Widget|RemovefromParent _notificationsuccess)
            (Variables|/Script/Engine.PlayerController|SetbShowMouseCursor _returnvalue_6 false)
            (Audio|PlaySound2D "/Game/SimpleUI/Sound/S_Click_Cue.S_Click_Cue")
            (Input|SetInputModeGameOnly _returnvalue_6)))))
    (:2
      ;[1 1 1] 2_Notification Warning
      (Utilities|FlowControl|Sequence
        (:then_0
          (if (Class|Button|IsPressed (Variables|/Game/SimpleUI/Blueprint/WidgetBlueprint/WG_Notification_Warning.WG_Notification_Warning_C|GetOKButton _notificationwarning))
            (Widget|RemovefromParent _notificationwarning)
            (Variables|/Script/Engine.PlayerController|SetbShowMouseCursor _returnvalue_3 false)
            (Audio|PlaySound2D "/Game/SimpleUI/Sound/S_Click_Cue.S_Click_Cue")
            (Input|SetInputModeGameOnly _returnvalue_3)))
        (:then_1
          (if (Class|Button|IsPressed (Variables|/Game/SimpleUI/Blueprint/WidgetBlueprint/WG_Notification_Warning.WG_Notification_Warning_C|GetCancelButton _notificationwarning))
            (Widget|RemovefromParent _notificationwarning)
            (Variables|/Script/Engine.PlayerController|SetbShowMouseCursor _returnvalue_4 false)
            (Audio|PlaySound2D "/Game/SimpleUI/Sound/S_Click_Cue.S_Click_Cue")
            (Input|SetInputModeGameOnly _returnvalue_4)))))
    (:3
      ;[1 1 1] 3_Scroll
      (Utilities|FlowControl|Sequence
        (:then_0
          (if (Class|Button|IsPressed (Variables|/Game/SimpleUI/Blueprint/WidgetBlueprint/WG_Scroll.WG_Scroll_C|GetOKButton _scroll))
            (Widget|RemovefromParent _scroll)
            (Variables|/Script/Engine.PlayerController|SetbShowMouseCursor _returnvalue_7 false)
            (Audio|PlaySound2D "/Game/SimpleUI/Sound/S_Click_Cue.S_Click_Cue")
            (Input|SetInputModeGameOnly _returnvalue_7)))
        (:then_1
          (if (Class|Button|IsPressed (Variables|/Game/SimpleUI/Blueprint/WidgetBlueprint/WG_Scroll.WG_Scroll_C|GetCancelButton _scroll))
            (Widget|RemovefromParent _scroll)
            (Variables|/Script/Engine.PlayerController|SetbShowMouseCursor _returnvalue_8 false)
            (Audio|PlaySound2D "/Game/SimpleUI/Sound/S_Click_Cue.S_Click_Cue")
            (Input|SetInputModeGameOnly _returnvalue_8)))))
    (:4
      ;[1 1 1] 4_TextInput
      (Utilities|FlowControl|Sequence
        (:then_0
          (if (Class|Button|IsPressed (Variables|/Game/SimpleUI/Blueprint/WidgetBlueprint/WG_TextInput.WG_TextInput_C|GetCancelButton _textinput))
            (Widget|RemovefromParent (Variables|Default|GetTextInput))
            (Variables|/Script/Engine.PlayerController|SetbShowMouseCursor _returnvalue_11 false)
            (Audio|PlaySound2D "/Game/SimpleUI/Sound/S_Click_Cue.S_Click_Cue")
            (Input|SetInputModeGameOnly _returnvalue_11)))
        (:then_1
          (if (Class|Button|IsPressed (Variables|/Game/SimpleUI/Blueprint/WidgetBlueprint/WG_TextInput.WG_TextInput_C|GetOKButton _textinput))
            (Rendering|Components|TextRender|SetText (Variables|Default|GetTextRender) (Class|EditableTextBox|GetText (Variables|/Game/SimpleUI/Blueprint/WidgetBlueprint/WG_TextInput.WG_TextInput_C|GetTextBox _textinput_2)))
            (Widget|RemovefromParent _textinput_2)
            (Variables|/Script/Engine.PlayerController|SetbShowMouseCursor _returnvalue_9 false)
            (Audio|PlaySound2D "/Game/SimpleUI/Sound/S_Click_Cue.S_Click_Cue")
            (Input|SetInputModeGameOnly _returnvalue_9)))))
    (:5
      (Utilities|FlowControl|Sequence
        (:then_0
          ;[1 1 1] 5-4_CubeRotation ( Toggle button )
          (if (UserInterface|Viewport|IsinViewport (Variables|Default|GetSetting))
            (if (not (Class|CheckBox|IsChecked (Variables|/Game/SimpleUI/Blueprint/WidgetBlueprint/WG_Setting.WG_Setting_C|GetToggleButton (Variables|Default|GetSetting))))
              ;[1 1 1] 5-3_Cube Rotation Speed ( Drop Down Box )
              (if (UserInterface|Viewport|IsinViewport (Variables|Default|GetSetting)) :!label _label
                (switch string (Class|ComboBoxString|GetSelectedOption (Variables|/Game/SimpleUI/Blueprint/WidgetBlueprint/WG_Setting.WG_Setting_C|GetDropDownBox (Variables|Default|GetSetting)))
                  (:VerySlow
                    (Variables|Default|SetSettingCubeSpeedTempValue 15.0))
                  (:Slow
                    (Variables|Default|SetSettingCubeSpeedTempValue 35.0))
                  (:Normal
                    (Variables|Default|SetSettingCubeSpeedTempValue 6e+01))
                  (:Fast
                    (Variables|Default|SetSettingCubeSpeedTempValue 5e+02))
                  (:VeryFast
                    (Variables|Default|SetSettingCubeSpeedTempValue 1e+03)))
                (Transformation|AddLocalRotation (Utilities|Array|MakeArray (Variables|Default|GetCube) (Variables|Default|GetCube2) (Variables|Default|GetCube3)) (Math|Rotator|MakeRotator 0.0 0.0 (* _returnvalue (Variables|Default|GetSettingCubeSpeedTempValue))) false false)
                (else
                  (Transformation|AddLocalRotation (Utilities|Array|MakeArray (Variables|Default|GetCube) (Variables|Default|GetCube2) (Variables|Default|GetCube3)) (Math|Rotator|MakeRotator 0.0 0.0 (* _returnvalue (Variables|Default|GetSettingCubeSpeedValue))) false false))))
            (elif (not (Variables|Default|GetToggleState))
              (goto _label))))
        (:then_1
          ;[1 1 1] 5-1_Cube Scale ( Slide Bar )
          (if (UserInterface|Viewport|IsinViewport (Variables|Default|GetSetting))
            (Transformation|SetRelativeScale3D (Utilities|Array|MakeArray (Variables|Default|GetCube) (Variables|Default|GetCube2) (Variables|Default|GetCube3)) (Math|Conversions|ToVector(Float) (+ (Class|Slider|GetValue (Variables|/Game/SimpleUI/Blueprint/WidgetBlueprint/WG_Setting.WG_Setting_C|GetSliderBar (Variables|Default|GetSetting))) 1.0)))
            (else
              (Transformation|SetRelativeScale3D (Utilities|Array|MakeArray (Variables|Default|GetCube) (Variables|Default|GetCube2) (Variables|Default|GetCube3)) (Math|Conversions|ToVector(Float) (+ (Variables|Default|GetSettingCubeScale) 1.0))))))
        (:then_2
          ;[1 1 1] 5-2_Cube Color ( Radio Button )
          (if (UserInterface|Viewport|IsinViewport (Variables|Default|GetSetting))
            (if (Class|CheckBox|IsChecked (Variables|/Game/SimpleUI/Blueprint/WidgetBlueprint/WG_Setting.WG_Setting_C|GetRadioButton1 (Variables|Default|GetSetting)))
              (Rendering|Material|SetMaterial _array 0 "/Game/SimpleUI/Materials/M_Cube.M_Cube")
              (else
                (Rendering|Material|SetMaterial _array 0 "/Game/SimpleUI/Materials/M_Cube2.M_Cube2")))
            (elif (Variables|Default|GetColorState)
              (Rendering|Material|SetMaterial _array_2 0 "/Game/SimpleUI/Materials/M_Cube.M_Cube")
              (else
                (Rendering|Material|SetMaterial _array_2 0 "/Game/SimpleUI/Materials/M_Cube2.M_Cube2")))))
        (:then_3
          ;[1 1 1] 5-5_Cube Visibility ( Check Box )
          (if (UserInterface|Viewport|IsinViewport (Variables|Default|GetSetting))
            (Development|SetHiddeninGame (Variables|Default|GetCube) (Utilities|Enum|Equal(Enum) (Class|CheckBox|GetCheckedState (Variables|/Game/SimpleUI/Blueprint/WidgetBlueprint/WG_Setting.WG_Setting_C|GetCheckBox1 (Variables|Default|GetSetting))) "Unchecked") false)
            (Development|SetHiddeninGame (Variables|Default|GetCube2) (Utilities|Enum|Equal(Enum) (Class|CheckBox|GetCheckedState (Variables|/Game/SimpleUI/Blueprint/WidgetBlueprint/WG_Setting.WG_Setting_C|GetCheckBox2 (Variables|Default|GetSetting))) "Unchecked") false)
            (Development|SetHiddeninGame (Variables|Default|GetCube3) (Utilities|Enum|Equal(Enum) (Class|CheckBox|GetCheckedState (Variables|/Game/SimpleUI/Blueprint/WidgetBlueprint/WG_Setting.WG_Setting_C|GetCheckBox3 (Variables|Default|GetSetting))) "Unchecked") false)
            (else
              (Development|SetHiddeninGame (Variables|Default|GetCube) (Variables|Default|GetCube1CheckState) false)
              (Development|SetHiddeninGame (Variables|Default|GetCube2) (Variables|Default|GetCube2CheckState) false)
              (Development|SetHiddeninGame (Variables|Default|GetCube3) (Variables|Default|GetCube3CheckState) false))))
        (:then_4
          ;[1 1 1] 5_Setting Accept Button - Applying the value entered by the user
          (if (Class|Button|IsPressed (Variables|/Game/SimpleUI/Blueprint/WidgetBlueprint/WG_Setting.WG_Setting_C|GetAcceptButton _setting))
            (CallFunction|SaveSettingCurrentValue)
            (Widget|RemovefromParent (Variables|Default|GetSetting))
            (Variables|/Script/Engine.PlayerController|SetbShowMouseCursor _returnvalue_10 false)
            (Audio|PlaySound2D "/Game/SimpleUI/Sound/S_Click_Cue.S_Click_Cue")
            (Input|SetInputModeGameOnly _returnvalue_10)))
        (:then_5
          ;[1 1 1] 5_Setting Default Button - The value is changed into the default value
          (if (Class|Button|IsPressed (Variables|/Game/SimpleUI/Blueprint/WidgetBlueprint/WG_Setting.WG_Setting_C|GetDefaultButton _setting))
            (CallFunction|GetSettingDefaultValue)
            (Audio|PlaySound2D "/Game/SimpleUI/Sound/S_Click_Cue.S_Click_Cue")))
        (:then_6
          ;[1 1 1] 5_Setting Cancel Button - The value is not changed
          (if (Class|Button|IsPressed (Variables|/Game/SimpleUI/Blueprint/WidgetBlueprint/WG_Setting.WG_Setting_C|GetCancelButton _setting))
            (Widget|RemovefromParent (Variables|Default|GetSetting))
            (Variables|/Script/Engine.PlayerController|SetbShowMouseCursor _returnvalue_13 false)
            (Audio|PlaySound2D "/Game/SimpleUI/Sound/S_Click_Cue.S_Click_Cue")
            (Input|SetInputModeGameOnly _returnvalue_13)))))))

(fn ConstructionScript)

(fn GetSettingCurrentValue
  (bind _setting (Variables|Default|GetSetting))
  (bind _togglebutton (Variables|/Game/SimpleUI/Blueprint/WidgetBlueprint/WG_Setting.WG_Setting_C|GetToggleButton _setting))
  (bind _checkbox1 (Variables|/Game/SimpleUI/Blueprint/WidgetBlueprint/WG_Setting.WG_Setting_C|GetCheckBox1 _setting))
  (bind _checkbox2 (Variables|/Game/SimpleUI/Blueprint/WidgetBlueprint/WG_Setting.WG_Setting_C|GetCheckBox2 _setting))
  (bind _checkbox3 (Variables|/Game/SimpleUI/Blueprint/WidgetBlueprint/WG_Setting.WG_Setting_C|GetCheckBox3 _setting))
  (Class|Slider|SetValue (Variables|/Game/SimpleUI/Blueprint/WidgetBlueprint/WG_Setting.WG_Setting_C|GetSliderBar _setting) (Variables|Default|GetSettingCubeScale))
  (if (Variables|Default|GetColorState)
    (Variables|Default|SetSettingCubeColor "Checked")
    (Variables|Default|SetSettingCubeColor2 "Unchecked")
    (else
      (Variables|Default|SetSettingCubeColor "Unchecked")
      (Variables|Default|SetSettingCubeColor2 "Checked")))
  (Class|CheckBox|SetCheckedState (Variables|/Game/SimpleUI/Blueprint/WidgetBlueprint/WG_Setting.WG_Setting_C|GetRadioButton1 _setting) (Variables|Default|GetSettingCubeColor))
  (Class|CheckBox|SetCheckedState (Variables|/Game/SimpleUI/Blueprint/WidgetBlueprint/WG_Setting.WG_Setting_C|GetRadioButtone2 _setting) (Variables|Default|GetSettingCubeColor2))
  (Class|ComboBoxString|SetSelectedOption (Variables|/Game/SimpleUI/Blueprint/WidgetBlueprint/WG_Setting.WG_Setting_C|GetDropDownBox _setting) (Variables|Default|GetSettingCubeSpeed))
  (if (Variables|Default|GetToggleState)
    (bind _output_get (Variables|Default|SetSettingRotation "Checked"))
    (Class|CheckBox|SetCheckedState _togglebutton _output_get)
    (else
      (bind _output_get_2 (Variables|Default|SetSettingRotation "Unchecked"))
      (Class|CheckBox|SetCheckedState _togglebutton _output_get_2)))
  (Class|CheckBox|SetCheckedState (Variables|/Game/SimpleUI/Blueprint/WidgetBlueprint/WG_Setting.WG_Setting_C|GetToggleButton _setting) (Variables|Default|GetSettingRotation))
  (if (Variables|Default|GetCube1CheckState)
    (bind _output_get_3 (Variables|Default|SetCube1Visibilty "Unchecked"))
    (Class|CheckBox|SetCheckedState _checkbox1 _output_get_3)
    (else
      (bind _output_get_4 (Variables|Default|SetCube1Visibilty "Checked"))
      (Class|CheckBox|SetCheckedState _checkbox1 _output_get_4)))
  (if (Variables|Default|GetCube2CheckState)
    (bind _output_get_5 (Variables|Default|SetCube2Visibilty "Unchecked"))
    (Class|CheckBox|SetCheckedState _checkbox2 _output_get_5)
    (else
      (bind _output_get_6 (Variables|Default|SetCube2Visibilty "Checked"))
      (Class|CheckBox|SetCheckedState _checkbox2 _output_get_6)))
  (if (Variables|Default|GetCube3CheckState)
    (bind _output_get_7 (Variables|Default|SetCube3Visibilty "Unchecked"))
    (Class|CheckBox|SetCheckedState _checkbox3 _output_get_7)
    (else
      (bind _output_get_8 (Variables|Default|SetCube3Visibilty "Checked"))
      (Class|CheckBox|SetCheckedState _checkbox3 _output_get_8))))

(fn SaveSettingCurrentValue
  (bind _setting (Variables|Default|GetSetting))
  (bind _radiobutton1 (Variables|/Game/SimpleUI/Blueprint/WidgetBlueprint/WG_Setting.WG_Setting_C|GetRadioButton1 _setting))
  (bind _togglebutton (Variables|/Game/SimpleUI/Blueprint/WidgetBlueprint/WG_Setting.WG_Setting_C|GetToggleButton _setting))
  (bind _checkbox1 (Variables|/Game/SimpleUI/Blueprint/WidgetBlueprint/WG_Setting.WG_Setting_C|GetCheckBox1 _setting))
  (bind _checkbox2 (Variables|/Game/SimpleUI/Blueprint/WidgetBlueprint/WG_Setting.WG_Setting_C|GetCheckBox2 _setting))
  (bind _checkbox3 (Variables|/Game/SimpleUI/Blueprint/WidgetBlueprint/WG_Setting.WG_Setting_C|GetCheckBox3 _setting))
  (bind _returnvalue (Class|CheckBox|GetCheckedState _checkbox1))
  (bind _returnvalue_2 (Class|CheckBox|GetCheckedState _checkbox2))
  (bind _returnvalue_3 (Class|CheckBox|GetCheckedState _checkbox3))
  (Variables|Default|SetSettingCubeScale (Class|Slider|GetValue (Variables|/Game/SimpleUI/Blueprint/WidgetBlueprint/WG_Setting.WG_Setting_C|GetSliderBar _setting)))
  (Variables|Default|SetSettingCubeColor (Class|CheckBox|GetCheckedState _radiobutton1))
  (Variables|Default|SetColorState (Class|CheckBox|IsChecked _radiobutton1))
  (Variables|Default|SetSettingCubeColor2 (Class|CheckBox|GetCheckedState (Variables|/Game/SimpleUI/Blueprint/WidgetBlueprint/WG_Setting.WG_Setting_C|GetRadioButtone2 _setting)))
  (bind _output_get (Variables|Default|SetSettingCubeSpeed (Class|ComboBoxString|GetSelectedOption (Variables|/Game/SimpleUI/Blueprint/WidgetBlueprint/WG_Setting.WG_Setting_C|GetDropDownBox _setting))))
  (switch string _output_get
    (:VerySlow
      (Variables|Default|SetSettingCubeSpeedValue 15.0))
    (:Slow
      (Variables|Default|SetSettingCubeSpeedValue 35.0))
    (:Normal
      (Variables|Default|SetSettingCubeSpeedValue 6e+01))
    (:Fast
      (Variables|Default|SetSettingCubeSpeedValue 5e+02))
    (:VeryFast
      (Variables|Default|SetSettingCubeSpeedValue 1e+03)))
  (Variables|Default|SetSettingRotation (Class|CheckBox|GetCheckedState _togglebutton))
  (Variables|Default|SetToggleState (Class|CheckBox|IsChecked _togglebutton))
  (Variables|Default|SetCube1Visibilty _returnvalue)
  (Variables|Default|SetCube1CheckState (Utilities|Enum|Equal(Enum) _returnvalue "Unchecked"))
  (Variables|Default|SetCube2Visibilty _returnvalue_2)
  (Variables|Default|SetCube2CheckState (Utilities|Enum|Equal(Enum) _returnvalue_2 "Unchecked"))
  (Variables|Default|SetCube3Visibilty _returnvalue_3)
  (Variables|Default|SetCube3CheckState (Utilities|Enum|Equal(Enum) _returnvalue_3 "Unchecked")))

(fn GetSettingDefaultValue
  (bind _setting (Variables|Default|GetSetting))
  (Class|Slider|SetValue (Variables|/Game/SimpleUI/Blueprint/WidgetBlueprint/WG_Setting.WG_Setting_C|GetSliderBar _setting) 0.0)
  (Class|CheckBox|SetCheckedState (Variables|/Game/SimpleUI/Blueprint/WidgetBlueprint/WG_Setting.WG_Setting_C|GetRadioButton1 _setting) "Checked")
  (Class|CheckBox|SetCheckedState (Variables|/Game/SimpleUI/Blueprint/WidgetBlueprint/WG_Setting.WG_Setting_C|GetRadioButtone2 _setting) "Unchecked")
  (Class|ComboBoxString|SetSelectedOption (Variables|/Game/SimpleUI/Blueprint/WidgetBlueprint/WG_Setting.WG_Setting_C|GetDropDownBox _setting) "Normal")
  (Class|CheckBox|SetCheckedState (Variables|/Game/SimpleUI/Blueprint/WidgetBlueprint/WG_Setting.WG_Setting_C|GetToggleButton _setting) "Unchecked")
  (Class|CheckBox|SetCheckedState (Variables|/Game/SimpleUI/Blueprint/WidgetBlueprint/WG_Setting.WG_Setting_C|GetCheckBox1 _setting) "Checked")
  (Class|CheckBox|SetCheckedState (Variables|/Game/SimpleUI/Blueprint/WidgetBlueprint/WG_Setting.WG_Setting_C|GetCheckBox2 _setting) "Unchecked")
  (Class|CheckBox|SetCheckedState (Variables|/Game/SimpleUI/Blueprint/WidgetBlueprint/WG_Setting.WG_Setting_C|GetCheckBox3 _setting) "Unchecked"))